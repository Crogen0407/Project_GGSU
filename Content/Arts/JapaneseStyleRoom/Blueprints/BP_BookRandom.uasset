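; Book-row scatter actor for the Japanese-style room that builds a line of randomly picked book meshes in its Construction Script.
; Each of the Num books gets its own static mesh component, spaced by Distance along local Y.
; With AlignZ, mesh bounds lift each book by its half-height, AlignY optionally shifts it by half-depth, and YawRotation sets roll.
; Otherwise, books receive random X and Z offsets and random pitch.
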(fn `UserConstructionScript`
  (locals (`Current Mesh` :type "StaticMesh Object Reference"))
  (bind _x_offset_random (`self.X Offset Random`))
  (bind _rotation_random (`self.Rotation Random`))
  (bind _y_offset_random (`self.Y Offset Random`))
  (bind (_returnvalue_origin _returnvalue_boxextent) (`KismetMathLibrary.BreakBoxSphereBounds` (`StaticMesh.GetBounds` (`local.Current Mesh`))))
  (for _index (range (`self.Num`))
    (if (`self.Align Z`)
      (set `local.Current Mesh` (`KismetArrayLibrary.Array_Random` (`self.Books`)))
      (bind _returnvalue (* _index (`self.Distance`)))
      (bind _returnvalue_2 (`AddComponent|NODE_AddStaticMeshComponent-1` :`RelativeTransform` (`KismetMathLibrary.MakeTransform` (`KismetMathLibrary.MakeVector` (`KismetMathLibrary.SelectFloat` (.x _returnvalue_boxextent) 0.0 (`self.Align Y`)) _returnvalue (.z _returnvalue_boxextent)) (`KismetMathLibrary.MakeRotator` (`self.Yaw Rotation`)))))
      (`StaticMeshComponent.SetStaticMesh` _returnvalue_2 (`local.Current Mesh`))
      (else
        (bind _returnvalue_3 (`AddComponent|NODE_AddStaticMeshComponent-0` :`RelativeTransform` (`KismetMathLibrary.MakeTransform` (`KismetMathLibrary.MakeVector` (`KismetMathLibrary.RandomFloatInRange` (* _x_offset_random -1.0) _x_offset_random) _returnvalue (`KismetMathLibrary.RandomFloatInRange` (* _y_offset_random -1.0) _y_offset_random)) (`KismetMathLibrary.MakeRotator` 0.0 (`KismetMathLibrary.RandomFloatInRange` (* _rotation_random -1.0) _rotation_random)))))
        (`StaticMeshComponent.SetStaticMesh` _returnvalue_3 (`KismetArrayLibrary.Array_Random` (`self.Books`)))))))